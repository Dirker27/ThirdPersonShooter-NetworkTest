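; Deprecated lit sliding door that characters open by interacting and that closes when they leave its trigger box.
; A timeline slides the door along relative Z, playing to open and reversing to close.
; SetColor tints both lights and a new emissive LightBar material instance for detection, opening and closing, and timeline completion restores the stored color and intensity.
; The OnRep handlers for color and intensity are empty.
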(event `self.ReceiveBeginPlay`
  (bind _rectlight2 (`self.RectLight2`))
  (set `self.LightColor` (`KismetMathLibrary.Conv_LinearColorToColor` (`LightComponentBase.GetLightColor` _rectlight2)))
  (set `self.LightIntensity` (`LightComponentBase.Intensity` _rectlight2)))

(event `self.Box.OnComponentBeginOverlap`
  (params (OverlappedComponent :type "PrimitiveComponent Object Reference") (OtherActor :type "Actor Object Reference") (OtherComp :type "PrimitiveComponent Object Reference") (OtherBodyIndex :type Integer) (bFromSweep :type Boolean) (SweepResult :type "HitResult Structure (by ref)"))
  (cast `Character` OtherActor)
  (`self.Detect Character`))

(event `Detect Character`
  (bind _output_get (set `self.LightColor` (`KismetMathLibrary.Conv_LinearColorToColor` (`KismetMathLibrary.MakeColor` 0.173 0.388 0.388))))
  (`self.SetColor` _output_get))

(event `/Game/TPS_Multiplayer/Door/BP_SlidingDoor_Interface.Interact`
  (params (Interactor :type "Pawn Object Reference"))
  (cast `Character` Interactor)
  (`self.OpenDoor`))

(event `OpenDoor`
  (`self.SetColor` (`KismetMathLibrary.Conv_LinearColorToColor` (`KismetMathLibrary.MakeColor` 0.49 0.604 0.267)))
  (bind (_direction _doorposition) (`Timeline|DoorOpening` :!label _label)
    (:`Update`
      (`SceneComponent.K2_SetRelativeLocation` (`self.Door`) (`KismetMathLibrary.MakeVector` 0.0 0.0 _doorposition) false false))
    (:`Finished`
      (`self.SetColor` (`self.LightColor`))
      (`self.SetIntensity` (`self.LightIntensity`)))))

(event `self.Box.OnComponentEndOverlap`
  (params (OverlappedComponent :type "PrimitiveComponent Object Reference") (OtherActor :type "Actor Object Reference") (OtherComp :type "PrimitiveComponent Object Reference") (OtherBodyIndex :type Integer))
  (cast `Character` OtherActor)
  (`self.CloseDoor`)
  (set `self.LightColor` (`KismetMathLibrary.Conv_LinearColorToColor` (`KismetMathLibrary.MakeColor` 1.0 1.0 1.0))))

(event `CloseDoor`
  (`self.SetColor` (`KismetMathLibrary.Conv_LinearColorToColor` (`KismetMathLibrary.MakeColor` 0.647 0.286 0.286)))
  (goto _label :!via `Reverse`))

(fn `OnRep_LightColor`)

(fn `OnRep_LightIntensity`)

(fn `SetColor`
  (params (Color :type "Color Structure"))
  (`LightComponent.SetLightColor` (`self.SpotLight`) (`KismetMathLibrary.Conv_ColorToLinearColor` Color) true)
  (`LightComponent.SetLightColor` (`self.RectLight2`) (`KismetMathLibrary.Conv_ColorToLinearColor` Color) true)
  (bind _returnvalue (`KismetMaterialLibrary.CreateDynamicMaterialInstance` "/Game/Common/Materials/M_EmissiveLight.M_EmissiveLight"))
  (`MaterialInstanceDynamic.SetVectorParameterValue` _returnvalue "Color" (`KismetMathLibrary.Conv_ColorToLinearColor` Color))
  (`PrimitiveComponent.SetMaterial` (`self.LightBar`) 0 _returnvalue)
  (return))

(fn `SetIntensity`
  (params (Intensity :type "Float (double-precision)"))
  (`LightComponent.SetIntensity` (`self.RectLight2`) Intensity)
  (`LightComponent.SetIntensity` (`self.SpotLight`) Intensity)
  (return))

(fn `UserConstructionScript`)