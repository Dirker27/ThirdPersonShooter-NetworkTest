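; Multiplayer sliding door that a character opens through Interact and that closes when a character leaves its box trigger while fully open.
; Timelines slide the door along Z between closed, opening, open and closing states, with locked states also handled.
; DoorState and IsCharacterDetected use OnReps to call SynchronizeDoorToState, which snaps settled positions and colors the light bar by state, using a different material when a character is detected.
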(event `self.ReceiveBeginPlay`
  (`self.SynchronizeDoorToState`))

(event `self.Box Collider.OnComponentBeginOverlap`
  (params (OverlappedComponent :type "PrimitiveComponent Object Reference") (OtherActor :type "Actor Object Reference") (OtherComp :type "PrimitiveComponent Object Reference") (OtherBodyIndex :type Integer) (bFromSweep :type Boolean) (SweepResult :type "HitResult Structure (by ref)"))
  ;[0.05098 0.05098 0.05098] Detect Character Entry
  (cast `Character` OtherActor)
  (`self.Detect Character`)
  (set `self.IsCharacterDetected` true :!label _label)
  (`self.SynchronizeDoorToState`))

(event `self.Box Collider.OnComponentEndOverlap`
  (params (OverlappedComponent :type "PrimitiveComponent Object Reference") (OtherActor :type "Actor Object Reference") (OtherComp :type "PrimitiveComponent Object Reference") (OtherBodyIndex :type Integer))
  ;[0.05098 0.05098 0.05098] Door Close on Timeout or All Characters Leave (Server Replicated)
  (cast `Character` OtherActor)
  (set `self.IsCharacterDetected` false)
  (if (`|EnumEquality` (`self.DoorState`) "NewEnumerator2")
    (set `self.DoorState` "NewEnumerator5")
    (`self.PerformCloseDoor`)
    (`self.SynchronizeDoorToState`)))

(event `Detect Character`
  ;[0.05098 0.05098 0.05098] Detect Character Entry
  (goto _label))

(event `PerformCloseDoor`
  ;[0.05098 0.05098 0.05098] Door Close on Timeout or All Characters Leave (Server Replicated)
  (bind (_direction _doorposition) (`Timeline|DoorClosing` :!via `PlayFromStart`)
    (:`Update`
      (`SceneComponent.K2_SetRelativeLocation` (`self.Sliding Door`) (`KismetMathLibrary.MakeVector` 0.0 0.0 _doorposition) false false))
    (:`Finished`
      (set `self.DoorState` "NewEnumerator0")
      (`self.SynchronizeDoorToState`))))

(event `/Game/TPS_Multiplayer/Props/Doors/BP_SlidingDoor_Interface.Interact`
  (params (Interactor :type "Pawn Object Reference"))
  ;[0.05098 0.05098 0.05098] Door Interaction (Server Replicated)
  (cast `Character` Interactor)
  (if (`|EnumEquality` (`self.DoorState`) "NewEnumerator0")
    (set `self.DoorState` "NewEnumerator4")
    (`self.PerformOpenDoor`)
    (`self.SynchronizeDoorToState`)))

(event `PerformOpenDoor`
  ;[0.05098 0.05098 0.05098] Door Open
  (bind (_direction _doorposition) (`Timeline|DoorOpening` :!via `PlayFromStart`)
    (:`Update`
      (`SceneComponent.K2_SetRelativeLocation` (`self.Sliding Door`) (`KismetMathLibrary.MakeVector` 0.0 0.0 _doorposition) false false))
    (:`Finished`
      (set `self.DoorState` "NewEnumerator2")
      (`self.SynchronizeDoorToState`))))

(fn `GetColorForState`
  (params (State :type "/Game/TPS_Multiplayer/Props/Doors/E_SlidingDoorState Enum" :default "NewEnumerator1"))
  (returns (Color :type "Color Structure"))
  (if (`|EnumEquality` State "NewEnumerator0")
    (return (`self.NeutralColor`))
    (elif (`|EnumEquality` State "NewEnumerator5")
      (return (`self.ClosingColor`))
      (elif (`|EnumEquality` State "NewEnumerator2")
        (return (`self.NeutralColor`))
        (elif (`|EnumEquality` State "NewEnumerator4")
          (return (`self.OpeningColor`))
          (elif (`|EnumEquality` State "NewEnumerator6")
            (return (`self.LockedColor`))
            (elif (`|EnumEquality` State "NewEnumerator1")
              (return (`self.LockedColor`)))))))))

(fn `OnRep_DoorState`
  (`self.SynchronizeDoorToState`))

(fn `OnRep_IsCharacterDetected`
  (`self.SynchronizeDoorToState`)
  (return))

(fn `SetColor`
  (params (Color :type "Color Structure"))
  (bind _returnvalue (`KismetMathLibrary.Conv_ColorToLinearColor` Color))
  (bind _lightbar (`self.LightBar`))
  (if (`self.IsCharacterDetected`)
    (bind _returnvalue_2 (`KismetMaterialLibrary.CreateDynamicMaterialInstance` "/Game/TPS_Multiplayer/Props/Doors/M_DoorLight_DetectedBrightness.M_DoorLight_DetectedBrightness"))
    (`MaterialInstanceDynamic.SetVectorParameterValue` _returnvalue_2 "Color" _returnvalue)
    (`PrimitiveComponent.SetMaterial` _lightbar 0 _returnvalue_2)
    (else
      (bind _returnvalue_3 (`KismetMaterialLibrary.CreateDynamicMaterialInstance` "/Game/TPS_Multiplayer/Props/Doors/M_DoorLight.M_DoorLight"))
      (`MaterialInstanceDynamic.SetVectorParameterValue` _returnvalue_3 "Color" _returnvalue)
      (`PrimitiveComponent.SetMaterial` _lightbar 0 _returnvalue_3)))
  (set `self.ActiveColor` Color)
  (return))

(fn `SynchronizeDoorToState`
  (bind _doorstate (`self.DoorState`))
  (`self.SetColor` (`self.GetColorForState` _doorstate))
  (if (`|EnumEquality` _doorstate "NewEnumerator4")
    _
    (elif (`|EnumEquality` _doorstate "NewEnumerator5")
      _
      (elif (`|EnumEquality` _doorstate "NewEnumerator2")
        (`SceneComponent.K2_SetRelativeLocation` (`self.Sliding Door`) (`KismetMathLibrary.MakeVector` 0.0 0.0 (`self.DoorDeltaZ`)) false false :!label _label)
        (elif (`|EnumEquality` _doorstate "NewEnumerator6")
          (goto _label)
          (elif (`|EnumEquality` _doorstate "NewEnumerator0")
            (`SceneComponent.K2_SetRelativeLocation` (`self.Sliding Door`) (0.0 0.0 0.0) false false :!label _label_2)
            (elif (`|EnumEquality` _doorstate "NewEnumerator1")
              (goto _label_2))))))))

(fn `UserConstructionScript`)